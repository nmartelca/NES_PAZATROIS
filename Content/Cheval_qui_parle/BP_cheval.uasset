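; BP_cheval is a talking horse that plays a sound and animates when its Cheval_qui_parle event is called.
; BeginPlay silences the Audio component and assigns it the Son sound.
; The event starts the audio and loops the walk animation on the Horse mesh, then switches to a looping idle after a fixed two-second delay, independent of the sound's length.
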(event `self.ReceiveBeginPlay`
  (`AudioComponent.StopDelayed` (`self.Audio`) 0.0)
  (`AudioComponent.SetSound` (`self.Audio`) (`self.Son`)))

(event `Cheval_qui_parle`
  (bind _horse (`self.Horse`))
  (`AudioComponent.Play` (`self.Audio`) 0.0)
  (`SkeletalMeshComponent.PlayAnimation` (`self.Horse`) "/Game/HorseStarterKit/Animation/Walk_Horse.Walk_Horse" true)
  (`KismetSystemLibrary.Delay` 2.0)
  (`SkeletalMeshComponent.Stop` _horse)
  (`SkeletalMeshComponent.PlayAnimation` _horse "/Game/HorseStarterKit/Animation/Idle_Horse.Idle_Horse" true))

(fn `UserConstructionScript`)